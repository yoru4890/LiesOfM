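; BP_TempEnemy is an enemy, apparently temporary, that periodically attacks BP_Yoru actors in front of it.
; On BeginPlay it caches its WB_EnemyHP health bar widget.
; Tick accumulates time and, about once per second, refreshes that widget and runs a debug-drawn multi-sphere trace forward from its static mesh.
; Each BP_Yoru hit receives fixed damage through ReceiveDamage, with the enemy as attacker.
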(event `self.ReceiveBeginPlay`
  (set `self.As WB Enemy HP` (cast `/Game/AAA/Widget/WB_EnemyHP` (`WidgetComponent.GetUserWidgetObject` (`self.HealthBar`)) :!pure true)))

(event `self.ReceiveTick`
  (params (DeltaSeconds :type "Float (single-precision)"))
  (bind _staticmesh (`self.StaticMesh`))
  (bind _returnvalue (+ (`self.deltaVector`) (`SceneComponent.K2_GetComponentLocation` _staticmesh)))
  (bind _output_get (set `self.elapsedTime` (+ DeltaSeconds (`self.elapsedTime`))))
  (if (>= _output_get 1.0)
    (set `self.elapsedTime` 0.0)
    (`/Game/AAA/Widget/WB_EnemyHP.RefreshHealthBar` (`self.As WB Enemy HP`) self)
    (bind (_outhits _returnvalue_2) (`KismetSystemLibrary.SphereTraceMulti` :`Start` _returnvalue :`End` (+ _returnvalue (* (`SceneComponent.GetForwardVector` _staticmesh) 1000.0)) :`TraceChannel` "TraceTypeQuery4" :`DrawDebugType` "ForDuration"))
    (if _returnvalue_2
      (for _array_element _outhits
        (bind (_bblockinghit _binitialoverlap _time _distance _location _impactpoint _normal _impactnormal _physmat _hitactor) (`GameplayStatics.BreakHitResult` _array_element))
        (if (`KismetMathLibrary.ClassIsChildOf` (`GameplayStatics.GetObjectClass` _hitactor) "/Game/AAA/Blueprints/Yoru/BP_Yoru.BP_Yoru_C")
          (`Yoru.ReceiveDamage` (cast `/Game/AAA/Blueprints/Yoru/BP_Yoru` _hitactor :!pure true) 10.0 self _array_element))))))

(fn `UserConstructionScript`)