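; Base wall actor that reacts to an effect at a given location with feedback matching its material.
; ReacttoEffect switches on ObjectProperty (steel, stone or wood) to spawn the matching Niagara system at that location.
; It also passes that material's sound array to PlaySound, which plays a random entry at the same spot.
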(event `HitEffectInterface.ReactToEffect`
  (params (location :type "Vector Structure"))
  (switch `/Game/AAA/Blueprints/Enum/E_ObjectProperty` (`self.objectProperty`)
    (:`NewEnumerator0`
      (`NiagaraFunctionLibrary.SpawnSystemAtLocation` "/Game/AAA/Effect/Niagara/NS_WallSteel.NS_WallSteel" location)
      (`self.PlaySound` location (`self.SteelSound`)))
    (:`NewEnumerator1`
      (`NiagaraFunctionLibrary.SpawnSystemAtLocation` "/Game/AAA/Effect/Niagara/NS_WallStone.NS_WallStone" location)
      (`self.PlaySound` location (`self.StoneSound`)))
    (:`NewEnumerator2`
      (`NiagaraFunctionLibrary.SpawnSystemAtLocation` "/Game/AAA/Effect/Niagara/NS_WallWood.NS_WallWood" location)
      (`self.PlaySound` location (`self.WoodSound`)))))

(fn `UserConstructionScript`)