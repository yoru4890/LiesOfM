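; Boss-door entry trigger that starts the boss encounter when the player character BP_Yoru overlaps its box.
; On the first visit recorded in the save game, it clears and saves that flag, hides the boss mesh and combat HUD, and plays an input-locking intro sequence.
; After a fixed delay it restores the HUD.
; Both first and repeat visits then call TriggerEnter and start the boss music.
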(event `self.ReceiveBeginPlay`
  (bind _asgm_truth_of_m (cast `/Game/AAA/GameMode/GM_TruthOfM` (`GameplayStatics.GetGameMode`)))
  (set `self.As GM Truth Of M` _asgm_truth_of_m)
  (bind _asbp_yoru (cast `/Game/AAA/Blueprints/Yoru/BP_Yoru` (`GameplayStatics.GetPlayerCharacter` 0)))
  (set `self.As BP Yoru` _asbp_yoru))

(event `self.Box.OnComponentBeginOverlap`
  (params (OverlappedComponent :type "PrimitiveComponent Object Reference") (OtherActor :type "Actor Object Reference") (OtherComp :type "PrimitiveComponent Object Reference") (OtherBodyIndex :type Integer) (bFromSweep :type Boolean) (SweepResult :type "HitResult Structure (by ref)"))
  (bind _as_gm_truth_of_m (`self.As GM Truth Of M`))
  (if (`KismetMathLibrary.ClassIsChildOf` (`GameplayStatics.GetObjectClass` OtherActor) "/Game/AAA/Blueprints/Yoru/BP_Yoru.BP_Yoru_C")
    (if (`/Game/AAA/SaveGame/SaveGame_TM.isBossFirstTime` (`/Game/AAA/GameMode/GM_TruthOfM.As Save Game TM` (`self.As GM Truth Of M`)))
      (`SceneComponent.SetVisibility` (`Character.Mesh` (`self.FFFBoss`)) false false)
      (`Widget.RemoveFromParent` (`YoruWidgetComponent.widgetCombat` (`Yoru.widgetComp` (`self.As BP Yoru`))))
      (set `/Game/AAA/SaveGame/SaveGame_TM.isBossFirstTime` false (`/Game/AAA/GameMode/GM_TruthOfM.As Save Game TM` _as_gm_truth_of_m))
      (`/Game/AAA/GameMode/GM_TruthOfM.SaveOut` _as_gm_truth_of_m)
      (bind (_outactor _returnvalue) (`LevelSequencePlayer.CreateLevelSequencePlayer` (`self.sequence`) (make `MovieSceneSequencePlaybackSettings` false (struct) 1.0 0.0 false false true true)))
      (`MovieSceneSequencePlayer.Play` _returnvalue)
      (`KismetSystemLibrary.Delay` 6.0)
      (`UserWidget.AddToViewport` (`YoruWidgetComponent.widgetCombat` (`Yoru.widgetComp` (`self.As BP Yoru`))) 0))
    (`self.TriggerEnter`)
    (bind _returnvalue_2 (`GameplayStatics.CreateSound2D` (`self.BossBGM`) 1.0 1.0 0.0 null))
    (bind _output_get (set `self.AudioControl` _returnvalue_2))
    (`AudioComponent.Play` _output_get 0.0)))

(fn `UserConstructionScript`)