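; Trigger volume at a boss door that lets the Yoru player character enter the boss area while standing inside it.
; On BeginPlay it caches the player as BP_Yoru and creates a WB_InterAction widget.
; Box overlap by a Yoru actor sets CanBossEnter on the player's MoveComp and shows the interaction widget; leaving clears the flag and removes it.
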(event `self.ReceiveBeginPlay`
  (`parent.ReceiveBeginPlay`)
  (bind _asbp_yoru (cast `/Game/AAA/Blueprints/Yoru/BP_Yoru` (`GameplayStatics.GetPlayerCharacter` 0)))
  (set `self.As BP Yoru` _asbp_yoru)
  (bind _returnvalue (`|CreateWidget` "/Game/AAA/Widget/WB_InterAction.WB_InterAction_C"))
  (set `self.InterActionWidget` _returnvalue))

(event `self.Box.OnComponentBeginOverlap`
  (params (OverlappedComponent :type "PrimitiveComponent Object Reference") (OtherActor :type "Actor Object Reference") (OtherComp :type "PrimitiveComponent Object Reference") (OtherBodyIndex :type Integer) (bFromSweep :type Boolean) (SweepResult :type "HitResult Structure (by ref)"))
  (if (`KismetMathLibrary.ClassIsChildOf` (`GameplayStatics.GetObjectClass` OtherActor) "/Script/LiesOfM.Yoru")
    (set `YoruMoveComponent.canBossEnter` true (`Yoru.moveComp` (`self.As BP Yoru`)))
    (`UserWidget.AddToViewport` (`self.InterActionWidget`) 0)))

(event `self.Box.OnComponentEndOverlap`
  (params (OverlappedComponent :type "PrimitiveComponent Object Reference") (OtherActor :type "Actor Object Reference") (OtherComp :type "PrimitiveComponent Object Reference") (OtherBodyIndex :type Integer))
  (if (`KismetMathLibrary.ClassIsChildOf` (`GameplayStatics.GetObjectClass` OtherActor) "/Script/LiesOfM.Yoru")
    (set `YoruMoveComponent.canBossEnter` false (`Yoru.moveComp` (`self.As BP Yoru`)))
    (`Widget.RemoveFromParent` (`self.InterActionWidget`))))

(fn `UserConstructionScript`
  (`parent.UserConstructionScript`))