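; BP_ElevatorLever is a trigger lever that activates its referenced Elevator when a Yoru actor overlaps its box.
; The overlap plays a gate sound and a timeline lowers the lever from its initial height.
; When lowered it activates the elevator, waits, then replays the sound and reverses the timeline to rise.
; UPState blocks retriggering from the end of the descent until the lever is back up.
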(event `self.ReceiveBeginPlay`
  (bind (_returnvalue_x _returnvalue_y _returnvalue_z) (`KismetMathLibrary.BreakVector` (`self.K2_GetActorLocation`)))
  (set `self.InitZ` _returnvalue_z))

(event `self.Box.OnComponentBeginOverlap`
  (params (OverlappedComponent :type "PrimitiveComponent Object Reference") (OtherActor :type "Actor Object Reference") (OtherComp :type "PrimitiveComponent Object Reference") (OtherBodyIndex :type Integer) (bFromSweep :type Boolean) (SweepResult :type "HitResult Structure (by ref)"))
  (bind (_returnvalue_x _returnvalue_y) (`KismetMathLibrary.BreakVector` (`self.K2_GetActorLocation`)))
  (if (`self.bUPState`)
    (if (`KismetMathLibrary.ClassIsChildOf` (`GameplayStatics.GetObjectClass` OtherActor) "/Script/LiesOfM.Yoru")
      (`GameplayStatics.PlaySoundAtLocation` "/Game/AAA/Audio/Door/stonegate.stonegate" (`self.K2_GetActorLocation`) (struct) 0.4 1.0 1.2 null null null null)
      (bind (_direction _newtrack_0) (`Timeline|Timeline` :!label _label)
        (:`Update`
          (`self.K2_SetActorLocation` (`KismetMathLibrary.MakeVector` _returnvalue_x _returnvalue_y (- (`self.InitZ`) _newtrack_0))))
        (:`Finished`
          (if (`self.bUPState`)
            (set `self.bUPState` false)
            (`/Game/AAA/Blueprints/Interface/BPI_Interact.Active` (`self.Elevator`))
            (`KismetSystemLibrary.Delay` 10.0)
            (`GameplayStatics.PlaySoundAtLocation` "/Game/AAA/Audio/Door/stonegate.stonegate" (`self.K2_GetActorLocation`) (struct) 0.4 1.0 1.2 null null null null)
            (goto _label :!via `Reverse`)
            (else
              (set `self.bUPState` true))))))))

(fn `UserConstructionScript`
  (`parent.UserConstructionScript`))