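; BP_Elevator_0 is an elevator actor that toggles between its start position and a timeline-driven end position when activated.
; Active plays a chain sound and runs the Timeline forward or in reverse, offsetting height and yaw from the BeginPlay transform, then flips UpState on finish.
; The construction script stacks Count chain meshes at a set spacing.
; ReacttoEffect spawns steel impact particles and a random steel sound.
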(event `self.ReceiveBeginPlay`
  (bind (_returnvalue_roll _returnvalue_pitch _returnvalue_yaw) (`KismetMathLibrary.BreakRotator` (`self.K2_GetActorRotation`)))
  (set `self.InitLocation` (`self.K2_GetActorLocation`))
  (set `self.InitYaw` _returnvalue_yaw))

(event `/Game/AAA/Blueprints/Interface/BPI_Interact.Active`
  (bind (_returnvalue_roll _returnvalue_pitch) (`KismetMathLibrary.BreakRotator` (`self.K2_GetActorRotation`)))
  (bind (_initlocation_x _initlocation_y _initlocation_z) (`KismetMathLibrary.BreakVector` (`self.InitLocation`)))
  (`GameplayStatics.PlaySoundAtLocation` "/Game/AAA/Audio/Door/slow-chain-drops.slow-chain-drops" (`self.K2_GetActorLocation`) (struct) 0.5 1.0 72.0 "/Game/AAA/Audio/Environment/SA_Rain.SA_Rain" null null null)
  (if (not (`self.bUpState`))
    (bind (_direction _newtrack_0 _newtrack_1) (`Timeline|Timeline` :!label _label)
      (:`Update`
        (`self.K2_SetActorLocationAndRotation` (`KismetMathLibrary.MakeVector` _initlocation_x _initlocation_y (+ _initlocation_z _newtrack_0)) (`KismetMathLibrary.MakeRotator` _returnvalue_roll _returnvalue_pitch (+ (`self.InitYaw`) _newtrack_1))))
      (:`Finished`
        (set `self.bUpState` (not (`self.bUpState`)))))
    (else
      (goto _label :!via `Reverse`))))

(event `HitEffectInterface.ReactToEffect`
  (params (location :type "Vector Structure"))
  (bind _steelsound (`self.SteelSound`))
  (`NiagaraFunctionLibrary.SpawnSystemAtLocation` "/Game/AAA/Effect/Niagara/NS_WallSteel.NS_WallSteel" location)
  (`GameplayStatics.PlaySoundAtLocation` (`|GetArrayItem` _steelsound (`KismetMathLibrary.RandomInteger` (`KismetArrayLibrary.Array_Length` _steelsound))) location (struct) 1.0 1.0 0.0 null null null null))

(fn `UserConstructionScript`
  (bind (_relativelocation_x _relativelocation_y _relativelocation_z) (`KismetMathLibrary.BreakVector` (`SceneComponent.RelativeLocation` (`self.SM_GDC2012_Throne_Interior_Chain_05`))))
  (`parent.UserConstructionScript`)
  (for _index (range 1 (+ (`self.Count`) 1))
    (`AddComponent|NODE_AddStaticMeshComponent-0` :`RelativeTransform` (`KismetMathLibrary.MakeTransform` (`KismetMathLibrary.MakeVector` _relativelocation_x _relativelocation_y (+ _relativelocation_z (* _index (`self.Distance`)))) (struct) (2.0 2.0 2.0)))))