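; BP_FallingDie is a trigger that kills the player character Yoru in a fall.
; On BeginPlay it casts player 0's character to BP_Yoru and caches the reference.
; When an actor of the Yoru class or a child enters the Box, it calls FallingDie on that cached character and makes the player controller ignore look input.
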(event `self.ReceiveBeginPlay`
  (`parent.ReceiveBeginPlay`)
  (bind _asbp_yoru (cast `/Game/AAA/Blueprints/Yoru/BP_Yoru` (`GameplayStatics.GetPlayerCharacter` 0)))
  (set `self.BPYoru` _asbp_yoru))

(event `self.Box.OnComponentBeginOverlap`
  (params (OverlappedComponent :type "PrimitiveComponent Object Reference") (OtherActor :type "Actor Object Reference") (OtherComp :type "PrimitiveComponent Object Reference") (OtherBodyIndex :type Integer) (bFromSweep :type Boolean) (SweepResult :type "HitResult Structure (by ref)"))
  (if (`KismetMathLibrary.ClassIsChildOf` (`GameplayStatics.GetObjectClass` OtherActor) "/Script/LiesOfM.Yoru")
    (`Yoru.FallingDie` (`self.BPYoru`))
    (`Controller.SetIgnoreLookInput` (`GameplayStatics.GetPlayerController` 0) true)))

(fn `UserConstructionScript`
  (`parent.UserConstructionScript`))