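; BP_Rain is a weather actor, presumably the rain effect, that hovers above the player character.
; On BeginPlay it caches the player as BP_Yoru and calls Active, a toggle that starts or clears a looping timer.
; While running, the timer repositions the actor at a fixed height over the player ten times a second, avoiding Tick.
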(event `self.ReceiveBeginPlay`
  (bind _asbp_yoru (cast `/Game/AAA/Blueprints/Yoru/BP_Yoru` (`GameplayStatics.GetPlayerCharacter` 0)))
  (set `self.BPYoru` _asbp_yoru)
  (`self.Active`))

(event `/Game/AAA/Blueprints/Interface/BPI_Follow.Active`
  (if (`self.bActive`)
    (set `self.bActive` false)
    (`KismetSystemLibrary.K2_ClearAndInvalidateTimerHandle` (`self.TimerHandle`))
    (else
      (set `self.bActive` true)
      (bind _returnvalue (`KismetSystemLibrary.K2_SetTimerDelegate` (delegate `FollowPlayer`) 0.1 true))
      (set `self.TimerHandle` _returnvalue))))

(event `FollowPlayer`
  (`self.K2_SetActorLocation` (+ (`self.K2_GetActorLocation` (`self.BPYoru`)) (0.0 0.0 2500.0))))

(fn `UserConstructionScript`
  (`parent.UserConstructionScript`))