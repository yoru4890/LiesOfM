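; BP_Yoru toggles the WB_Option options menu when Tab or Escape is pressed.
; It creates the widget on first use, caches it in WidgetOption, and uses IsRendered to decide whether to show or remove it.
; Showing the menu switches to UI-only input with a visible cursor, and removing it restores game-only input and hides the cursor.
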(event `self.ReceiveBeginPlay`)

(event `self.ReceiveTick`
  (params (DeltaSeconds :type "Float (single-precision)")))

(event `Key|Tab`
  (params (Key :type "Key Structure"))
  (bind _returnvalue (`GameplayStatics.GetPlayerController` 0))
  (bind _returnvalue_2 (`GameplayStatics.GetPlayerController` 0))
  (:`Pressed`
    (`/Engine/EditorBlueprintResources/StandardMacros.IsValid` (`self.WidgetOption`) :!label _label
      (:`Is Valid`
        (if (`Widget.IsRendered` (`self.WidgetOption`))
          (`Widget.RemoveFromParent` (`self.WidgetOption`))
          (`WidgetBlueprintLibrary.SetInputMode_GameOnly` _returnvalue)
          (set `PlayerController.bShowMouseCursor` false _returnvalue)
          (else
            (`UserWidget.AddToViewport` (stale _output_get) 0 :!label _label_2)
            (`WidgetBlueprintLibrary.SetInputMode_UIOnlyEx` _returnvalue_2 null)
            (set `PlayerController.bShowMouseCursor` true _returnvalue_2))))
      (:`Is Not Valid`
        (bind _returnvalue_3 (`|CreateWidget` "/Game/AAA/Widget/WB_Option.WB_Option_C"))
        (bind _output_get (set `self.WidgetOption` _returnvalue_3))
        (goto _label_2)))))

(event `Key|Escape`
  (params (Key :type "Key Structure"))
  (:`Pressed`
    (goto _label)))

(fn `UserConstructionScript`)