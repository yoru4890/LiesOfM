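; GM_TruthOfM is the game mode that creates or loads the save game and restores the BP_Yoru player's location.
; On BeginPlay it caches the player pawn and game instance, then creates a fresh SaveGame_TM if none exists or IsNewGame is set, clearing that flag.
; Otherwise it loads the slot and moves the player to the saved location.
; SaveLocation stores a given location and writes it to the slot.
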(event `self.ReceiveBeginPlay`
  (`|ExecutionSequence`
    (:`then_0`
      (bind _asbp_yoru (cast `/Game/AAA/Blueprints/Yoru/BP_Yoru` (`GameplayStatics.GetPlayerPawn` 0)))
      (set `self.As BP Yoru` _asbp_yoru)
      (bind _asgi_tomgame_instance (cast `/Game/AAA/GameMode/GI_TOMGameInstance` (`GameplayStatics.GetGameInstance`)))
      (set `self.As GI TOMGame Instance` _asgi_tomgame_instance))
    (:`then_1`
      (bind _returnvalue (`GameplayStatics.DoesSaveGameExist` (`self.SaveSlotName`)))
      (if _returnvalue
        (if (`/Game/AAA/GameMode/GI_TOMGameInstance.isNewGame` (`self.As GI TOMGame Instance`))
          (bind _returnvalue_2 (`GameplayStatics.CreateSaveGameObject` "/Game/AAA/SaveGame/SaveGame_TM.SaveGame_TM_C" :!label _label))
          (set `self.As Save Game TM` _returnvalue_2)
          (set `/Game/AAA/GameMode/GI_TOMGameInstance.isNewGame` false (`self.As GI TOMGame Instance`))
          (else
            (bind _returnvalue_3 (`GameplayStatics.LoadGameFromSlot` (`self.SaveSlotName`)))
            (bind _assave_game_tm (cast `/Game/AAA/SaveGame/SaveGame_TM` _returnvalue_3))
            (set `self.As Save Game TM` _assave_game_tm)
            (`self.InitPlayer`)))
        (else
          (goto _label))))))

(event `InitPlayer`
  (`self.K2_SetActorLocation` (`self.As BP Yoru`) (`/Game/AAA/SaveGame/SaveGame_TM.PlayerLocation` (`self.As Save Game TM`)) false false))

(event `SaveLocation`
  (params (Loc :type "Vector Structure"))
  (set `/Game/AAA/SaveGame/SaveGame_TM.PlayerLocation` Loc (`self.As Save Game TM`))
  (`self.SaveOut`))

(event `SaveOut`
  (`GameplayStatics.SaveGameToSlot` (`self.As Save Game TM`) (`self.SaveSlotName`)))

(fn `UserConstructionScript`)