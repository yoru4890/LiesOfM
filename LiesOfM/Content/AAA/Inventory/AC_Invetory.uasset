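; Inventory component that toggles the WB_InventoryTool widget on screen when the I key is pressed.
; BeginPlay adds the IMC_Yoru mapping context, and the first press creates, caches and shows the widget.
; Later presses flip-flop between InventoryClose, with removal after a one-second delay, and InventoryOpen with re-adding to the viewport.
; Mouse cursor and input mode switch between game-only and game-and-UI accordingly.
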(event `self.ReceiveBeginPlay`
  (`EnhancedInputSubsystemInterface.AddMappingContext` (pcsubsystem `EnhancedInputLocalPlayerSubsystem` (`GameplayStatics.GetPlayerController` 0)) "/Game/AAA/Input/IMC_Yoru.IMC_Yoru" 0 (struct)))

(event `Key|I`
  (params (Key :type "Key Structure"))
  (bind _returnvalue (`GameplayStatics.GetPlayerController` 0))
  (bind _returnvalue_2 (`GameplayStatics.GetPlayerController` 0))
  (bind _inventorytool (`self.InventoryTool`))
  (:`Pressed`
    (`self.InventoryTool`
      (:`then`
        (`/Engine/EditorBlueprintResources/StandardMacros.FlipFlop`
          (:`A`
            (`/Game/AAA/Inventory/WB_InventoryTool.Inventory Close` _inventorytool)
            (`KismetSystemLibrary.Delay` 1.0)
            (`Widget.RemoveFromParent` _inventorytool)
            (set `PlayerController.bShowMouseCursor` false _returnvalue_2)
            (`WidgetBlueprintLibrary.SetInputMode_GameOnly` _returnvalue_2))
          (:`B`
            (`/Game/AAA/Inventory/WB_InventoryTool.Inventory Open` (`self.InventoryTool`))
            (`UserWidget.AddToViewport` (`self.InventoryTool`) 0)
            (set `PlayerController.bShowMouseCursor` true _returnvalue_2)
            (`WidgetBlueprintLibrary.SetInputMode_GameAndUIEx` _returnvalue_2 null))))
      (:`else`
        (bind _returnvalue_3 (`|CreateWidget` "/Game/AAA/Inventory/WB_InventoryTool.WB_InventoryTool_C" (`GameplayStatics.GetPlayerController` 0)))
        (bind _output_get (set `self.InventoryTool` _returnvalue_3))
        (`UserWidget.AddToViewport` _output_get 0)
        (`WidgetBlueprintLibrary.SetInputMode_GameAndUIEx` _returnvalue null)
        (set `PlayerController.bShowMouseCursor` true _returnvalue)))))